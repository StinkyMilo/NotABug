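; BP_Web is a web object that slows BaseCharacter actors inside its sphere.
; Overlap begin and end events add and remove characters from CharactersInWeb, with a debug print on entry.
; Each tick overwrites the capsule's physics linear velocity of each tracked character with its current velocity scaled by SlowdownPercentage.
; An unconnected sphere trace sketches an unfinished idea for distance-based slowdown.
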(event OnComponentBeginOverlap(WebSphere)
  (params (OverlappedComponent :type Primitive%20Component%20Object%20Reference) (OtherActor :type Actor%20Object%20Reference) (OtherComp :type Primitive%20Component%20Object%20Reference) (OtherBodyIndex :type Integer) (bFromSweep :type Boolean) (SweepResult :type Hit%20Result%20Structure%20%28by%20ref%29))
  ;[0.4336 1 0.6957] when something enters the web
  (bind _asbase_character (Utilities|Casting|CastToBaseCharacter OtherActor))
  (Utilities|Array|Add (Variables|Default|GetCharactersInWeb) _asbase_character)
  (Development|PrintText (Utilities|Text|FormatText "web collided with {testThing}" (Utilities|GetClassDisplayName (Utilities|GetClass OtherActor))) true false))

(event OnComponentEndOverlap(WebSphere)
  (params (OverlappedComponent :type Primitive%20Component%20Object%20Reference) (OtherActor :type Actor%20Object%20Reference) (OtherComp :type Primitive%20Component%20Object%20Reference) (OtherBodyIndex :type Integer))
  ;[1 0.2395 0.2495] when something exits the web
  (bind _asbase_character (Utilities|Casting|CastToBaseCharacter OtherActor))
  (Utilities|Array|RemoveItem (Variables|Default|GetCharactersInWeb) _asbase_character))

(event EventTick
  (params (DeltaSeconds :type Float%20%28single-precision%29))
  ;[0.3408 0.6547 1] every tick, update velocity of all actors in web
  (for _array_element (Variables|Default|GetCharactersInWeb)
    (Class|PrimitiveComponent|SetAllPhysicsLinearVelocity (Variables|/Game/Game/Players/Character/BaseCharacter.BaseCharacter_C|GetCapsule _array_element) (* (Variables|Default|GetSlowdownPercentage) (Transformation|GetVelocity _array_element)) false)))

(fn ConstructionScript)