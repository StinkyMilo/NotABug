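; BP_AimSpline is a spline-mesh actor, named as an aiming visual for the player's web objects, that starts scaled down and hidden.
; The construction script adds one Y-forward spline mesh per segment between spline points and stores them in an array.
; Tick re-fits each stored mesh to the current local point locations and tangents, relying on the point count never changing.
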(event EventBeginPlay
  (Transformation|SetActorScale3D "0.050000,0.050000,0.050000")
  (Rendering|SetVisibility (Variables|Transformation|GetRootComponent) false true))

(event Collision|EventActorBeginOverlap
  (params (OtherActor :type Actor%20Object%20Reference)))

(event EventTick
  (params (DeltaSeconds :type Float%20%28single-precision%29))
  (bind _spline (Variables|Default|GetSpline))
  ;[1 1 1] not as good as it could be visually, but it works because the # of points will always equal the # of mesh components
  (for _index (range 0 (- (Spline|GetNumberOfSplinePoints (Variables|Default|GetSpline)) 2))
    (SplineMesh|SetStartandEnd (Utilities|Array|Get(acopy) (Variables|Default|GetSplineMeshComponents) _index) (.Location (Spline|GetLocationandTangentatSplinePoint _spline _index "Local")) (.Tangent (Spline|GetLocationandTangentatSplinePoint _spline _index "Local")) (.Location (Spline|GetLocationandTangentatSplinePoint _spline (+ _index 1) "Local")) (.Tangent (Spline|GetLocationandTangentatSplinePoint _spline (+ _index 1) "Local")) true :!class /Script/Engine.SplineMeshComponent)))

(fn ConstructionScript
  (bind _spline (Variables|Default|GetSpline))
  (for _index (range 0 (- (Spline|GetNumberOfSplinePoints (Variables|Default|GetSpline)) 2))
    (bind _returnvalue (AddComponent|AddSplineMeshComponent false))
    (SplineMesh|SetForwardAxis _returnvalue "Y" true)
    (SplineMesh|SetStartandEnd _returnvalue (.Location (Spline|GetLocationandTangentatSplinePoint _spline _index "Local")) (.Tangent (Spline|GetLocationandTangentatSplinePoint _spline _index "Local")) (.Location (Spline|GetLocationandTangentatSplinePoint _spline (+ _index 1) "Local")) (.Tangent (Spline|GetLocationandTangentatSplinePoint _spline (+ _index 1) "Local")) true :!class /Script/Engine.SplineMeshComponent)
    (Utilities|Array|Add (Variables|Default|GetSplineMeshComponents) _returnvalue)))