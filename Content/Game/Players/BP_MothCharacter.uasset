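; Moth player character that can jump repeatedly, including in mid-air, because its CanJumpInternal override always returns true.
; Each Jump press calls Jump immediately, clears a CanJump flag and restarts a delay timer.
; Tick counts the timer down and restores the flag, but the branch that would gate jumping on it is disconnected, so the cooldown has no effect.
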(event EventTick
  (params (DeltaSeconds :type Float%20%28single-precision%29))
  (if (not (Variables|Default|GetCanJump?))
    (bind _output_get (Variables|Default|SetJumpFTimer (- (Variables|Default|GetJumpFTimer) DeltaSeconds)))
    (if (<= _output_get 0.0)
      (Variables|Default|SetCanJump? true))))

(event Input|ActionEvents|InputActionJump
  (params (Key :type Key%20Structure :default "None"))
  (:Pressed
    (Character|Jump)
    (Variables|Default|SetCanJump? false)
    (Variables|Default|SetJumpFTimer (Variables|Default|GetJumpDelay))))

(fn ConstructionScript
  (|CallParentFunction))

(fn CanJumpInternal
  (return true))