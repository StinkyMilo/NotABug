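; Trigger volume actor that opens a menu once both the Moth and Spider characters have entered its box.
; Begin overlap matches the other actor's exact class to set a per-character flag, then a DoOnce pushes the configured widget onto the BugGameMode widget stack when both are set.
; End overlap is meant to clear the flags, but its class checks have no actor input.
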(event OnComponentBeginOverlap(Box)
  (params (OverlappedComponent :type Primitive%20Component%20Object%20Reference) (OtherActor :type Actor%20Object%20Reference) (OtherComp :type Primitive%20Component%20Object%20Reference) (OtherBodyIndex :type Integer) (bFromSweep :type Boolean) (SweepResult :type Hit%20Result%20Structure%20%28by%20ref%29))
  (bind _returnvalue (Utilities|GetClass OtherActor))
  (if (== _returnvalue "/Game/Game/Players/Character/Character_Moth.Character_Moth_C")
    (Variables|Default|SetMoth? true)
    (if (and (Variables|Default|GetSpider?) (Variables|Default|GetMoth?)) :!label _label
      (Utilities|FlowControl|DoOnce false
        (:Completed
          (CallFunction|PushWidgetOfType (Variables|/Game/Game/BugGameMode.BugGameMode_C|GetWidget%20Stack (.AsBug%20Game%20Mode (Utilities|Casting|CastToBugGameMode (Game|GetGameMode)))) (Variables|Default|GetWidget)))))
    (elif (== _returnvalue "/Game/Game/Players/Character/Character_Spider.Character_Spider_C")
      (Variables|Default|SetSpider? true)
      (goto _label))))

(event OnComponentEndOverlap(Box)
  (params (OverlappedComponent :type Primitive%20Component%20Object%20Reference) (OtherActor :type Actor%20Object%20Reference) (OtherComp :type Primitive%20Component%20Object%20Reference) (OtherBodyIndex :type Integer))
  (bind _returnvalue (Utilities|GetClass 0))
  (if (== _returnvalue "/Game/Game/Players/Character/Character_Moth.Character_Moth_C")
    (Variables|Default|SetMoth? false)
    (elif (== _returnvalue "/Game/Game/Players/Character/Character_Spider.Character_Spider_C")
      (Variables|Default|SetSpider? false))))

(event EventBeginPlay)

(event Collision|EventActorBeginOverlap
  (params (OtherActor :type Actor%20Object%20Reference)))

(event EventTick
  (params (DeltaSeconds :type Float%20%28single-precision%29)))

(fn ConstructionScript)