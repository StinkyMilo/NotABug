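; BP_VisibilityTrigger is a one-shot box trigger that swaps the visibility of assigned actors and can start dialogue.
; On BeginPlay it hides every actor in ToEnable.
; The first overlap of any actor shows ToEnable, hides ToDisable, then plays DialogueToPlay, if valid, through the BugGameMode dialogue manager, using that dialogue's PauseControls setting.
; It changes only hidden-in-game state.
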(event OnComponentBeginOverlap(Box)
  (params (OverlappedComponent :type Primitive%20Component%20Object%20Reference) (OtherActor :type Actor%20Object%20Reference) (OtherComp :type Primitive%20Component%20Object%20Reference) (OtherBodyIndex :type Integer) (bFromSweep :type Boolean) (SweepResult :type Hit%20Result%20Structure%20%28by%20ref%29))
  (bind _dialoguetoplay (Variables|Default|GetDialogueToPlay))
  (Utilities|FlowControl|DoOnce false
    (:Completed
      (Utilities|FlowControl|Sequence
        (:then_0
          (for _array_element (Variables|Default|GetToEnable)
            (Rendering|SetActorHiddenInGame _array_element false)))
        (:then_1
          (for _array_element_2 (Variables|Default|GetToDisable)
            (Rendering|SetActorHiddenInGame _array_element_2 true)))
        (:then_2
          (Utilities|IsValid (Variables|Default|GetDialogueToPlay)
            (:Is%20Valid
              (bind _asbug_game_mode (Utilities|Casting|CastToBugGameMode (Game|GetGameMode)))
              (Default|PlayDialogueExchange (Variables|/Game/Game/BugGameMode.BugGameMode_C|GetBPC_DialogueManager _asbug_game_mode) _dialoguetoplay (Variables|/Game/Game/UI/Dialogue/DataTypes/DA_DialogueObject.DA_DialogueObject_C|GetPauseControls _dialoguetoplay) false))))))))

(event EventBeginPlay
  (for _array_element (Variables|Default|GetToEnable)
    (Rendering|SetActorHiddenInGame _array_element true)))

(fn ConstructionScript)