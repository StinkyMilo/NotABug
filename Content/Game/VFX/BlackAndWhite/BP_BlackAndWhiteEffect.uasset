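; BP_BlackAndWhiteEffect is an unfinished Blueprint, apparently meant as a black-and-white screen effect through camera saturation.
; On BeginPlay it waits one tick, then caches the active camera from the CameraManager on BP_BugGameInstance.
; SetSaturation does nothing: its post-process settings nodes are left disconnected, so the cached camera's image is never changed.
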(event EventBeginPlay
  (Utilities|FlowControl|DelayUntilNextTick)
  (Variables|Default|SetCamera (Variables|/Game/CameraStuff/CameraManager.CameraManager_C|GetActiveCamera (Variables|/Game/Game/BP_BugGameInstance.BP_BugGameInstance_C|GetCameraManager (.AsBP%20Bug%20Game%20Instance (Utilities|Casting|CastToBP_BugGameInstance (Game|GetGameInstance)))))))

(event Collision|EventActorBeginOverlap
  (params (OtherActor :type Actor%20Object%20Reference)))

(event EventTick
  (params (DeltaSeconds :type Float%20%28single-precision%29)))

(fn ConstructionScript)

(fn SetSaturation
  (params (Saturation :type Float%20%28double-precision%29)))