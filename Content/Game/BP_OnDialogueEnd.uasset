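; BP_OnDialogueEnd is a level actor that reacts when a specific dialogue exchange finishes.
; On BeginPlay it binds to the game mode's dialogue manager end event and deactivates the root components of the actors in ToEnable.
; When the watched dialogue ends, it reactivates those components, destroys the ToDisable actors and, if set, plays a follow-up dialogue without pausing controls.
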(event Custom|On%20Receive
  (params (FinishedDialogueExchange :type DA%20Dialogue%20Object%20Object%20Reference))
  (bind _dialoguetoplay (Variables|Default|GetDialogueToPlay))
  (if (== FinishedDialogueExchange (Variables|Default|GetDialougeToListenTo))
    (Utilities|FlowControl|Sequence
      (:then_0
        (for _array_element (Variables|Default|GetToEnable)
          (Components|Activation|Activate (Variables|/Script/Engine.Actor|GetRootComponent _array_element) false)))
      (:then_1
        (for _array_element_2 (Variables|Default|GetToDisable)
          (Actor|DestroyActor _array_element_2)))
      (:then_2
        (Utilities|IsValid _dialoguetoplay
          (:Is%20Valid
            (bind _asbug_game_mode (Utilities|Casting|CastToBugGameMode (Game|GetGameMode)))
            (Default|PlayDialogueExchange (Variables|/Game/Game/BugGameMode.BugGameMode_C|GetBPC_DialogueManager _asbug_game_mode) _dialoguetoplay false false)))))))

(event EventBeginPlay
  (EventDispatchers|BindEventtoOnDialogueEnd (Variables|/Game/Game/BugGameMode.BugGameMode_C|GetBPC_DialogueManager (.AsBug%20Game%20Mode (Utilities|Casting|CastToBugGameMode (Game|GetGameMode)))) (delegate Custom|On%20Receive))
  (for _array_element (Variables|Default|GetToEnable)
    (Components|Activation|Deactivate (Variables|/Script/Engine.Actor|GetRootComponent _array_element))))

(fn ConstructionScript)