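; BP_LightBlocker is an actor with a cube that fades out once a dialogue ends, presumably to stop blocking light.
; On BeginPlay it binds to the game mode's dialogue manager and gives the cube a dynamic M_FadeGradually material.
; Any dialogue end starts the fade, and Tick then lowers the Opacity parameter by Speed toward zero.
; The cube is never destroyed or hidden, and Tick keeps updating after reaching zero.
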(event Custom|StartFade
  (Variables|Default|SetFade? true))

(event Custom|OnDIalogue
  (params (FinishedDialogueExchange :type %20Object%20Reference))
  (CallFunction|StartFade))

(event EventTick
  (params (DeltaSeconds :type Float%20%28single-precision%29))
  (if (Variables|Default|GetFade?)
    (bind _output_get (Variables|Default|SetOpacity (Math|Float|Clamp(Float) (- (Variables|Default|GetOpacity) (* DeltaSeconds (Variables|Default|GetSpeed))))))
    (bind _asmaterial_instance_dynamic (Utilities|Casting|CastToMaterialInstanceDynamic (Rendering|Material|GetMaterial (Variables|Default|GetCube) 0)))
    (Rendering|Material|SetScalarParameterValue (Variables|Default|GetMaterial) "Opacity" _output_get :!class /Script/Engine.MaterialInstanceDynamic)
    (if (== (Variables|Default|GetOpacity) 0.0)
      _)))

(event EventBeginPlay
  (EventDispatchers|BindEventtoOnDialogueEnd (Variables|/Game/Game/BugGameMode.BugGameMode_C|GetBPC_DialogueManager (.AsBug%20Game%20Mode (Utilities|Casting|CastToBugGameMode (Game|GetGameMode)))) (delegate Custom|OnDIalogue))
  (bind _returnvalue (Rendering|Material|CreateDynamicMaterialInstance "/Game/Game/M_FadeGradually.M_FadeGradually" "None" "None" :!class /Script/Engine.KismetMaterialLibrary))
  (Rendering|Material|SetMaterial (Variables|Default|GetCube) 0 _returnvalue)
  (Variables|Default|SetMaterial _returnvalue))

(fn ConstructionScript)